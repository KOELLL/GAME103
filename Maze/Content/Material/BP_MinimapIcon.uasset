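; BP_MinimapIcon is a minimap marker actor that follows a target actor from a fixed height.
; On BeginPlay it scales its static mesh by IconScale in X and Y and flattens it in Z.
; Each Tick it moves to the TargetActor's X and Y at IconHeight, and destroys itself once that target is no longer valid.
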(event `self.ReceiveBeginPlay`
  (`SceneComponent.SetRelativeScale3D` (`self.StaticMesh`) (`KismetMathLibrary.MakeVector` (`self.IconScale`) (`self.IconScale`) 0.05)))

(event `self.ReceiveTick`
  (params (DeltaSeconds :type "Float (single-precision)"))
  (bind _targetactor (`self.TargetActor`))
  (`/Engine/EditorBlueprintResources/StandardMacros.IsValid` _targetactor
    (:`Is Valid`
      (`self.K2_SetActorLocation` (`KismetMathLibrary.MakeVector` (.x (`self.K2_GetActorLocation` _targetactor)) (.y (`self.K2_GetActorLocation` _targetactor)) (`self.Icon Height`))))
    (:`Is Not Valid`
      (`self.K2_DestroyActor`))))

(fn `UserConstructionScript`)