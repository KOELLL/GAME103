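; Maze enemy character that patrols the generated maze and chases the player on sight, damaging and speed-boosting them when it catches them.
; Patrol loops AI moves to random locations supplied by the maze generator that initializes it.
; Pawn sensing starts a chase that rechecks distance and time since last sighting after each move, reverting to patrol when either limit is exceeded.
; State changes set walk speed and switch the generator's background music.
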(event `InitializeEnemy`
  (params (Generator :type "/Game/Maze/BP_MazeGenerator Object Reference"))
  (set `self.MazeGeneratorRef_0` Generator)
  (`self.ChangeEnemyState` "NewEnumerator1")
  (`KismetSystemLibrary.Delay` 0.5)
  (`self.StartPatrol`))

(event `StartPatrol`
  (bind _mazegeneratorref_0 (`self.MazeGeneratorRef_0`))
  (if (`|EnumEquality` (`self.EnemyState`) "NewEnumerator1")
    (`/Engine/EditorBlueprintResources/StandardMacros.IsValid` _mazegeneratorref_0
      (:`Is Valid`
        (bind (_success _patrollocation) (`/Game/Maze/BP_MazeGenerator.GetRandomEnemyPatrolLocation` _mazegeneratorref_0))
        (if _success
          (`|AIMoveTo` self _patrollocation null 80.0
            (:`OnSuccess`
              (`KismetSystemLibrary.Delay` 1.0)
              (`self.StartPatrol`))
            (:`OnFail`
              (`KismetSystemLibrary.Delay` 0.5)
              (`self.StartPatrol`))))))))

(event `self.PawnSensing.OnSeePawn`
  (params (Pawn :type "Pawn Object Reference"))
  (set `self.TargetPlayer` Pawn)
  (set `self.LastSeenPlayerTime` (`KismetSystemLibrary.GetGameTimeInSeconds`))
  (if (`|EnumInequality` (`self.EnemyState`) "NewEnumerator2")
    (`self.ChangeEnemyState` "NewEnumerator2")
    (`Controller.StopMovement` (`self.GetController`))
    (`self.ChasePlayer`)))

(event `ChasePlayer`
  (if (`|EnumEquality` (`self.EnemyState`) "NewEnumerator2")
    (if (`KismetSystemLibrary.IsValid` (`self.TargetPlayer`))
      (`|AIMoveTo` self (0.0 0.0 0.0) (`self.TargetPlayer`) 120.0
        (:`OnSuccess`
          (set `self.LastSeenPlayerTime` (`KismetSystemLibrary.GetGameTimeInSeconds`))
          (`KismetSystemLibrary.PrintString` "Caught Player")
          (bind _asbp_first_person_character (cast `/Game/FirstPerson/Blueprints/BP_FirstPersonCharacter` (`self.TargetPlayer`)))
          (`GameplayStatics.PlaySound2D` "/Game/Sound/grunt_001.grunt_001" 1.0 1.0 0.0 null null)
          (`GameplayStatics.PlaySound2D` "/Game/Sound/Attack_sound.Attack_sound" 1.0 1.0 0.0 null null)
          (`/Game/FirstPerson/Blueprints/BP_FirstPersonCharacter.TriggerSpeedBoost` _asbp_first_person_character)
          (`/Game/FirstPerson/Blueprints/BP_FirstPersonCharacter.TakeCaughtDamage` _asbp_first_person_character)
          (`KismetSystemLibrary.Delay` 2.0)
          (`self.CheckChaseValid`))
        (:`OnFail`
          (`KismetSystemLibrary.Delay` 0.3)
          (`self.CheckChaseValid`)))
      (else
        (`self.ReturnToPatrol`)))))

(event `CheckChaseValid`
  (if (`|EnumEquality` (`self.EnemyState`) "NewEnumerator2")
    (if (`KismetSystemLibrary.IsValid` (`self.TargetPlayer`))
      (if (and (<= (`KismetMathLibrary.Vector_Distance` (`self.K2_GetActorLocation`) (`self.K2_GetActorLocation` (`self.TargetPlayer`))) (`self.ChaseMaxDistance`)) (<= (- (`KismetSystemLibrary.GetGameTimeInSeconds`) (`self.LastSeenPlayerTime`)) (`self.LostSightDelay`)))
        (`self.ChasePlayer`)
        (else
          (`self.ReturnToPatrol`))))))

(event `ReturnToPatrol`
  (set `self.TargetPlayer` null)
  (`self.ChangeEnemyState` "NewEnumerator1")
  (`Controller.StopMovement` (`self.GetController`))
  (`KismetSystemLibrary.Delay` 0.3)
  (`self.StartPatrol`))

(event `ChangeEnemyState`
  (params (NewState :type "/Game/Maze/Enum_EnemyState Enum" :default "NewEnumerator0"))
  (bind _charactermovement (`self.CharacterMovement`))
  (bind _mazegeneratorref_0 (`self.MazeGeneratorRef_0`))
  (bind _output_get (set `self.EnemyState` NewState))
  (switch `/Game/Maze/Enum_EnemyState` _output_get
    (:`NewEnumerator1`
      (set `CharacterMovementComponent.MaxWalkSpeed` 200.0 _charactermovement)
      (`/Game/Maze/BP_MazeGenerator.SetBGMState` _mazegeneratorref_0 "NewEnumerator1"))
    (:`NewEnumerator2`
      (set `CharacterMovementComponent.MaxWalkSpeed` 550.0 _charactermovement)
      (`/Game/Maze/BP_MazeGenerator.SetBGMState` _mazegeneratorref_0 "NewEnumerator2"))))

(fn `UserConstructionScript`)