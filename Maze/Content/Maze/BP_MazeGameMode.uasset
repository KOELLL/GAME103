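; Game mode for a maze run in which the player gathers collectibles, then escapes to win.
; A phase enum gates each step: InitializeRun stores the target and maze generator, and RegisterCollectible tallies count and score.
; Reaching the target starts the escape phase through the generator's BeginEscapePhase.
; WinGame then locks player move and look input; its level-load node never runs.
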(fn `InitializeRun`
  (params (TargetCount :type Integer) (GeneratorRef :type "/Game/Maze/BP_MazeGenerator Object Reference"))
  (set `self.TargetCollectibles` TargetCount)
  (set `self.CollectedCount` 0)
  (set `self.Score` 0)
  (bind _output_get (set `self.MazeGeneratorRef` GeneratorRef))
  (`/Engine/EditorBlueprintResources/StandardMacros.IsValid` _output_get
    (:`Is Valid`
      (set `self.GamePhase` "NewEnumerator1")
      (`KismetSystemLibrary.PrintString` "Maze Run Initialized")
      (`KismetSystemLibrary.PrintString` (`KismetStringLibrary.Conv_IntToString` (`self.TargetCollectibles`))))))

(fn `RegisterCollectible`
  (params (Value :type Integer))
  (if (`|EnumEquality` (`self.GamePhase`) "NewEnumerator1")
    (bind _output_get (set `self.CollectedCount` (+ (`self.CollectedCount`) 1)))
    (`KismetSystemLibrary.PrintString` (`KismetStringLibrary.Conv_IntToString` _output_get))
    (bind _output_get_2 (set `self.Score` (+ (`self.Score`) Value)))
    (`KismetSystemLibrary.PrintString` (`KismetStringLibrary.Conv_IntToString` _output_get_2))
    (if (>= _output_get (`self.TargetCollectibles`))
      (`self.StartEscapePhase`))))

(fn `StartEscapePhase`
  (bind _mazegeneratorref (`self.MazeGeneratorRef`))
  (if (`|EnumEquality` (`self.GamePhase`) "NewEnumerator1")
    (set `self.GamePhase` "NewEnumerator2")
    (`/Engine/EditorBlueprintResources/StandardMacros.IsValid` _mazegeneratorref
      (:`Is Valid`
        (`/Game/Maze/BP_MazeGenerator.BeginEscapePhase` _mazegeneratorref))
      (:`Is Not Valid`
        (`KismetSystemLibrary.PrintString` "MazeGeneratorRef Invalid")))))

(fn `UserConstructionScript`)

(fn `WinGame`
  (bind _returnvalue (`GameplayStatics.GetPlayerController` 0))
  (if (`|EnumEquality` (`self.GamePhase`) "NewEnumerator2")
    (set `self.GamePhase` "NewEnumerator3")
    (`Controller.SetIgnoreMoveInput` _returnvalue true)
    (`Controller.SetIgnoreLookInput` _returnvalue true)
    (`KismetSystemLibrary.PrintString` "Escaped")))