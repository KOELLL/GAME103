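; BP_ExitPortal is the maze exit, which starts hidden with its trigger box collision off.
; ActivateExit sets the ExitActive flag, shows the mesh without propagating to its children, enables query-only collision and prints a message.
; Once active, a BP_FirstPersonCharacter overlapping the box calls WinGame on BP_MazeGameMode.
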(event `self.ReceiveBeginPlay`
  (`SceneComponent.SetVisibility` (`self.StaticMesh`) false true)
  (`PrimitiveComponent.SetCollisionEnabled` (`self.Box`) "NoCollision"))

(event `self.Box.OnComponentBeginOverlap`
  (params (OverlappedComponent :type "PrimitiveComponent Object Reference") (OtherActor :type "Actor Object Reference") (OtherComp :type "PrimitiveComponent Object Reference") (OtherBodyIndex :type Integer) (bFromSweep :type Boolean) (SweepResult :type "HitResult Structure (by ref)"))
  (if (`self.ExitActive`)
    (cast `/Game/FirstPerson/Blueprints/BP_FirstPersonCharacter` OtherActor)
    (bind _asbp_maze_game_mode (cast `/Game/Maze/BP_MazeGameMode` (`GameplayStatics.GetGameMode`)))
    (`/Game/Maze/BP_MazeGameMode.WinGame` _asbp_maze_game_mode)))

(fn `ActivateExit`
  (set `self.ExitActive` true)
  (`SceneComponent.SetVisibility` (`self.StaticMesh`) true false)
  (`PrimitiveComponent.SetCollisionEnabled` (`self.Box`) "QueryOnly")
  (`KismetSystemLibrary.PrintString` "EXIT ACTIVATED"))

(fn `UserConstructionScript`)