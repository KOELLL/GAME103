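; BP_Collectible is a maze pickup that awards points when the player's first-person character touches it.
; A Sphere overlap casts to BP_FirstPersonCharacter, then uses a Collected flag and disabled collision so it only counts once.
; It reports its PointValue to BP_MazeGameMode via RegisterCollectible, plays a 2D sound and destroys itself.
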(event `self.StaticMesh.OnComponentBeginOverlap`
  (params (OverlappedComponent :type "PrimitiveComponent Object Reference") (OtherActor :type "Actor Object Reference") (OtherComp :type "PrimitiveComponent Object Reference") (OtherBodyIndex :type Integer) (bFromSweep :type Boolean) (SweepResult :type "HitResult Structure (by ref)")))

(event `self.Sphere.OnComponentBeginOverlap`
  (params (OverlappedComponent :type "PrimitiveComponent Object Reference") (OtherActor :type "Actor Object Reference") (OtherComp :type "PrimitiveComponent Object Reference") (OtherBodyIndex :type Integer) (bFromSweep :type Boolean) (SweepResult :type "HitResult Structure (by ref)"))
  (`KismetSystemLibrary.PrintString` "Collectible Overlap")
  (cast `/Game/FirstPerson/Blueprints/BP_FirstPersonCharacter` OtherActor)
  (if (not (`self.Collected`))
    (set `self.Collected` true)
    (`PrimitiveComponent.SetCollisionEnabled` (`self.Sphere`) "NoCollision")
    (bind _asbp_maze_game_mode (cast `/Game/Maze/BP_MazeGameMode` (`GameplayStatics.GetGameMode`)))
    (`/Game/Maze/BP_MazeGameMode.RegisterCollectible` _asbp_maze_game_mode (`self.PointValue`))
    (`GameplayStatics.PlaySound2D` "/Game/Sound/Modern4.Modern4" 1.0 1.0 0.0 null null)
    (`self.K2_DestroyActor`)))

(fn `UserConstructionScript`)